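; BP_Switch is a one-way switch actor that reveals a set of light actors when interacted with.
; On BeginPlay it loops over its Lights array and hides each actor in game.
; The Interact event loops over the same array and unhides them, with no logic to switch them back off.
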(event `self.ReceiveBeginPlay`
  (for _array_element (`self.Lights`)
    (`self.SetActorHiddenInGame` _array_element true)))

(event `/Game/BP/Inventory/InteractionInterface.Interact`
  (for _array_element (`self.Lights`)
    (`self.SetActorHiddenInGame` _array_element false)))

(fn `UserConstructionScript`
  (`parent.UserConstructionScript`))
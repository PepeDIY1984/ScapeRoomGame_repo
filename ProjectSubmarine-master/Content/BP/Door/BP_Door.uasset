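; BP_Door is a door with a three-value combination lock, worked from a close-up camera mode.
; Camera activation enables input and shows the DoorHUB widget, where movement keys turn a dial in ten-degree steps.
; ConfirmKey checks each value in order, counting errors and resetting once attempts run out.
; The final match exits the camera through the player component and swings the door open via a timeline.
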(event `/Game/BP/Inventory/InteractionInterface.Interact`
  (`GameplayStatics.SpawnSoundAttached` "/Engine/VREditor/Sounds/UI/Dockable_Window_Pick_Up.Dockable_Window_Pick_Up" (`self.Cube`) "None" (0.0 0.0 0.0) (struct) "KeepRelativeOffset" false 1.0 1.0 0.0 null null))

(event `InputAxis|RotateActor`
  (params (AxisValue :type "Float (single-precision)"))
  ; Activate Rotation
)

(event `InputAction|Movement1`
  (params (Key :type "Key Structure"))
  ; Activate Rotation
  (:`Pressed`
    (`/Engine/EditorBlueprintResources/StandardMacros.IsValid` (`self.PlayerComponent`)
      (:`Is Valid`
        (if (and (`self.CameraChange`) (not (`/Game/FirstPerson/Blueprints/BP_FirstPersonCharacter.InInventory` (`self.PlayerComponent`))))
          (bind _output_get (set `self.CurrentRotation` (+ (`self.CurrentRotation`) 10.0)))
          (`self.TextPosition` _output_get)
          (`SceneComponent.K2_SetRelativeRotation` (`self.StaticMesh_0`) (`KismetMathLibrary.MakeRotator` 0.0 _output_get) false false)
          (`GameplayStatics.PlaySoundAtLocation` "/Game/Sounds/003_hatch.003_hatch" (`SceneComponent.K2_GetComponentLocation` (`self.StaticMesh_0`)) (struct) 1.0 1.0 0.0 null null null null :!label _label))))))

(event `InputAction|Movement-1`
  (params (Key :type "Key Structure"))
  ; Activate Rotation
  (:`Pressed`
    (`/Engine/EditorBlueprintResources/StandardMacros.IsValid` (`self.PlayerComponent`)
      (:`Is Valid`
        (if (and (`self.CameraChange`) (not (`/Game/FirstPerson/Blueprints/BP_FirstPersonCharacter.InInventory` (`self.PlayerComponent`))))
          (bind _output_get (set `self.CurrentRotation` (- (`self.CurrentRotation`) 10.0)))
          (`self.TextPosition` _output_get)
          (`SceneComponent.K2_SetRelativeRotation` (`self.StaticMesh_0`) (`KismetMathLibrary.MakeRotator` 0.0 _output_get) false false)
          (goto _label))))))

(event `EventCameraActiv`
  (params (Player_Component :type "/Game/FirstPerson/Blueprints/BP_FirstPersonCharacter Object Reference"))
  ; Event Camera Activ
  (set `self.PlayerComponent` Player_Component)
  (`self.EnableInput` (`GameplayStatics.GetPlayerController` 0))
  (bind _returnvalue (`|CreateWidget` "/Game/Widget/DoorHUB.DoorHUB_C"))
  (bind _output_get (set `self.DoorHub` _returnvalue))
  (set `self.CameraChange` true)
  (`UserWidget.AddToViewport` _output_get 0)
  (`self.TextPosition` (`self.CurrentRotation`)))

(event `EventCameraDeact`
  (bind _doorhub (`self.DoorHub`))
  ; Event Camera Activ
  (`self.DisableInput` (`GameplayStatics.GetPlayerController` 0))
  (set `self.CameraChange` false)
  (`/Engine/EditorBlueprintResources/StandardMacros.IsValid` _doorhub
    (:`Is Valid`
      (`Widget.RemoveFromParent` _doorhub)
      (set `self.CurrentRotation` 0.0)
      (`SceneComponent.K2_SetRelativeRotation` :`self` (`self.StaticMesh_0`)))))

(event `InputAction|ConfirmKey`
  (params (Key :type "Key Structure"))
  (bind _output (`|GetArrayItem` (`self.Combination`) (`self.PointCombination`)))
  ; Confirm Key
  (:`Pressed`
    (`/Engine/EditorBlueprintResources/StandardMacros.IsValid` (`self.PlayerComponent`)
      (:`Is Valid`
        (if (not (`/Game/FirstPerson/Blueprints/BP_FirstPersonCharacter.InInventory` (`self.PlayerComponent`)))
          (set `self.CombinationEvaluation` _output)
          (if (<= (`self.Attempts`) 3)
            (if (and (== _output (`self.CurrentRotation`)) (not (`self.CombinationComplete`)))
              (if (== (`self.PointCombination`) 0)
                (`self.SoundSuccess`)
                (`TextBlock.SetText` (`/Game/Widget/DoorHUB.TextBlock_Key1` (`self.DoorHub`)) (`KismetTextLibrary.Conv_DoubleToText` (`self.CombinationEvaluation`) "HalfToEven"))
                (set `self.PointCombination` (+ (`self.PointCombination`) 1) :!label _label_2)
                (elif (== (`self.PointCombination`) 1)
                  (`self.SoundSuccess`)
                  (`TextBlock.SetText` (`/Game/Widget/DoorHUB.TextBlock_Key2` (`self.DoorHub`)) (`KismetTextLibrary.Conv_DoubleToText` (`self.CombinationEvaluation`) "HalfToEven"))
                  (goto _label_2)
                  (elif (== (`self.PointCombination`) 2)
                    (`self.SoundSuccess`)
                    (`TextBlock.SetText` (`/Game/Widget/DoorHUB.TextBlock_Key3` (`self.DoorHub`)) (`KismetTextLibrary.Conv_DoubleToText` (`self.CombinationEvaluation`) "HalfToEven"))
                    ; End
                    (set `self.CombinationComplete` true)
                    (set `/Game/Widget/DoorHUB.Visibilityunlocking` true (`self.DoorHub`))
                    (`KismetSystemLibrary.Delay` 1.0)
                    (set `/Game/Widget/DoorHUB.Visibilityunlocking` false (`self.DoorHub`))
                    (`/Game/FirstPerson/Blueprints/BP_FirstPersonCharacter.Camera change` (`self.PlayerComponent`))
                    (`self.OpenDoor`)
                    (set `self.HideText` true))))
              (else
                (`GameplayStatics.PlaySoundAtLocation` "/Game/Sounds/002_Error.002_Error" (`SceneComponent.K2_GetComponentLocation` (`self.StaticMesh_0`)) (struct) 1.0 1.0 0.0 null null null null)
                (set `self.Attempts` (+ (`self.Attempts`) 1))))
            (else
              (`self.Reset`))))))))

(event `Reset`
  ; Reset for error
  (`TextBlock.SetText` (`/Game/Widget/DoorHUB.TextBlock_Key1` (`self.DoorHub`)) "0.0")
  (`TextBlock.SetText` (`/Game/Widget/DoorHUB.TextBlock_Key2` (`self.DoorHub`)) "0.0")
  (`TextBlock.SetText` (`/Game/Widget/DoorHUB.TextBlock_Key3` (`self.DoorHub`)) "0.0")
  (`SceneComponent.K2_SetRelativeRotation` :`self` (`self.StaticMesh_0`))
  (set `self.Attempts` 0)
  (set `self.PointCombination` 0)
  (set `self.CurrentRotation` 0.0)
  (`self.TextPosition` 0.0))

(event `OpenDoor`
  ; Custom Event Open Door
  (`/Engine/EditorBlueprintResources/StandardMacros.FlipFlop`
    (:`A`
      (bind (_direction _animdoor) (`Timeline|TL_OpenDoor` :!label _label_3)
        (:`Update`
          (`SceneComponent.K2_SetRelativeRotation` (`self.Arrow`) (`KismetMathLibrary.MakeRotator` 0.0 0.0 (`KismetMathLibrary.Lerp` (`self.DoorClosed`) (`self.DoorOpen`) _animdoor)) false false))))
    (:`B`
      (goto _label_3 :!via `Reverse`))))

(fn `SoundSuccess`
  (`GameplayStatics.PlaySoundAtLocation` "/Game/Sounds/001_Success.001_Success" (`SceneComponent.K2_GetComponentLocation` (`self.StaticMesh_0`)) (struct) 1.0 1.0 0.0 null null null null)
  (return))

(fn `TextPosition`
  (params (Position :type "Float (double-precision)"))
  (`TextBlock.SetText` (`/Game/Widget/DoorHUB.TextBlock_0` (`self.DoorHub`)) (`KismetTextLibrary.Conv_StringToText` (`KismetStringLibrary.Conv_DoubleToString` Position)))
  (return))

(fn `UserConstructionScript`
  (`parent.UserConstructionScript`))
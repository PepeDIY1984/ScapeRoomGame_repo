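; Base interactable item pickup that adds its InformationItem to the first-person character on interaction.
; The construction script sets the mesh from that item data and configures the Box and Sphere volumes.
; Show and reset message events swap the highlight material and display the HUD prompt once per reset, while enable and disable events toggle Sphere collision and prompt visibility.
; Interacting also enables flashlight flicker, plays a pickup sound and destroys the actor.
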(event `Enable Interact`
  (`PrimitiveComponent.SetCollisionEnabled` (`self.Sphere`) "QueryAndPhysics")
  (setmembers `/Game/BP/Inventory/LookAtInteractStructure` :`StructRef` (`self.InteractConfig`) :`ShowHUD` true))

(event `Disable Interact`
  (`PrimitiveComponent.SetCollisionEnabled` (`self.Sphere`) "NoCollision")
  (setmembers `/Game/BP/Inventory/LookAtInteractStructure` :`StructRef` (`self.InteractConfig`) :`ShowHUD` false))

(event `ShowInteractionMessage`
  (params (BP_Interaction :type "/Game/BP/Inventory/BP_InteractionParent Object Reference"))
  (`self.MaterialOn`)
  (if (not (`self.HideText`))
    (`/Engine/EditorBlueprintResources/StandardMacros.DoOnce` false :!label _label
      (:`Completed`
        (`/Game/Widget/InteractHUB.ShowInteractHUB` (`/Game/FirstPerson/Blueprints/BP_FirstPersonCharacter.PlayerHUB` (cast `/Game/FirstPerson/Blueprints/BP_FirstPersonCharacter` (`GameplayStatics.GetPlayerCharacter` 0) :!pure true)) (`KismetTextLibrary.Conv_StringToText` (`.InteractText_6_E9A40E904D8C1BE19718A681CE65916E` (break `/Game/BP/Inventory/LookAtInteractStructure` (`self.InteractConfig`)))))))))

(event `ResetMessage`
  (params (`BP Interaction` :type "/Game/BP/Inventory/BP_InteractionParent Object Reference"))
  (`self.MaterialOff`)
  (goto _label :!via `Reset`))

(event `/Game/BP/Inventory/InteractionInterface.Deinteract`)

(event `MaterialOn`
  (`PrimitiveComponent.SetMaterial` (`self.Model`) 0 "/Engine/VREditor/UI/ArrowMaterial.ArrowMaterial"))

(event `MaterialOff`
  (`PrimitiveComponent.SetMaterial` (`self.Model`) 0 "/Engine/BasicShapes/BasicShapeMaterial.BasicShapeMaterial"))

(event `/Game/BP/Inventory/InteractionInterface.Interact`
  (bind _asbp_first_person_character (cast `/Game/FirstPerson/Blueprints/BP_FirstPersonCharacter` (`GameplayStatics.GetPlayerCharacter` 0)))
  (set `/Game/FirstPerson/Blueprints/BP_FirstPersonCharacter.FlashlightFlickerEnable` true _asbp_first_person_character)
  (`/Game/FirstPerson/Blueprints/BP_FirstPersonCharacter.AddItem` _asbp_first_person_character (`self.InformationItem`))
  (`GameplayStatics.PlaySoundAtLocation` "/Game/Sounds/007_PickUp.007_PickUp" (0.0 0.0 0.0) (struct) 1.0 1.0 0.0 null null (`GameplayStatics.GetPlayerCharacter` 0) null)
  (`KismetSystemLibrary.Delay` 0.2)
  (`self.K2_DestroyActor` self))

(fn `GetInformationComplete`)

(fn `UserConstructionScript`
  (bind _box (`self.Box`))
  (bind (_informationitem_keyitem _informationitem_name _informationitem_description _informationitem_image _informationitem_row _informationitem_model) (break `/Game/BP/Inventory/S_ItemComplete` (`self.InformationItem`)))
  (`BoxComponent.SetBoxExtent` _box (`self.In Box Extent`) true)
  (`SphereComponent.SetSphereRadius` (`self.Sphere`) (`self.In Sphere Radius`) true)
  (`SceneComponent.K2_SetWorldRotation` _box (`self.New Rotation`) false false)
  (`SceneComponent.K2_SetRelativeLocation` _box (`self.New Location`) false false)
  (`StaticMeshComponent.SetStaticMesh` (`self.Model`) _informationitem_model))
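; BP_CameraObject is an inventory preview actor that shows an item mesh alongside a SceneCaptureComponent2D and lets it be rotated.
; UpdateStaticMesh applies the passed item's mesh, moves the capture camera to its position and stores its min/max position bounds, which are not used here.
; RotateObject combines roll and pitch input, scaled by RotationSpeed and the delta time cached on Tick, into the mesh's relative rotation.
; ResetMesh clears the mesh.
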(event `self.ReceiveTick`
  (params (DeltaSeconds :type "Float (single-precision)"))
  (set `self.Delta Seconds` DeltaSeconds))

(fn `ResetMesh`
  (`StaticMeshComponent.SetStaticMesh` (`self.StaticMesh`) null))

(fn `RotateObject`
  (params (RotationX :type "Float (double-precision)") (RotationY :type "Float (double-precision)"))
  (bind (_returnvalue_roll _returnvalue_pitch) (`KismetMathLibrary.BreakRotator` (`KismetMathLibrary.MakeRotator` RotationX RotationY)))
  (`SceneComponent.K2_SetRelativeRotation` (`self.StaticMesh`) (`KismetMathLibrary.ComposeRotators` (`SceneComponent.RelativeRotation` (`self.StaticMesh`)) (`KismetMathLibrary.MakeRotator` (* (* _returnvalue_roll (`self.RotationSpeed`)) (`self.Delta Seconds`)) (* (* _returnvalue_pitch (`self.RotationSpeed`)) (`self.Delta Seconds`)))) false false))

(fn `UpdateMaxPosition`
  (params (MinPosition :type "Float (double-precision)") (MaxPosition :type "Float (double-precision)"))
  (set `self.MinPosition` MinPosition)
  (set `self.MaxPosition` MaxPosition))

(fn `UpdateStaticMesh`
  (params (NewParam :type "/Game/BP/Inventory/S_Recording Structure"))
  (bind (_mesh _cameraposition _maxposition _minposition) (break `/Game/BP/Inventory/S_Recording` NewParam))
  (`StaticMeshComponent.SetStaticMesh` (`self.StaticMesh`) _mesh)
  (`SceneComponent.K2_SetRelativeLocation` (`self.SceneCaptureComponent2D`) _cameraposition false false)
  (`self.UpdateMaxPosition` _minposition _maxposition))

(fn `UserConstructionScript`)
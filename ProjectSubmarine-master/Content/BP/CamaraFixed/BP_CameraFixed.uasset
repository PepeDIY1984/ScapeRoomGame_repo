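; BP_CameraFixed is an interactive fixed-view actor that takes over the player's view when its Box is overlapped, with no check on what overlapped.
; Overlap blends the view to this actor and enables the cursor and click events.
; Pressing Q blends back to BP_FirstPersonCharacter and disables both.
; Clicking Button prints a debug message and uses a FlipFlop with MoveComponentTo to toggle it between two relative heights.
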(event `self.ReceiveBeginPlay`
  (`self.EnableInput` (`GameplayStatics.GetPlayerController` 0)))

(event `self.Box.OnComponentBeginOverlap`
  (params (OverlappedComponent :type "PrimitiveComponent Object Reference") (OtherActor :type "Actor Object Reference") (OtherComp :type "PrimitiveComponent Object Reference") (OtherBodyIndex :type Integer) (bFromSweep :type Boolean) (SweepResult :type "HitResult Structure (by ref)"))
  (bind _returnvalue (`GameplayStatics.GetPlayerController` 0))
  (`PlayerController.SetViewTargetWithBlend` _returnvalue self 0.5 "VTBlend_Linear" 0.0 false)
  (set `PlayerController.bEnableClickEvents` true _returnvalue)
  (set `PlayerController.bShowMouseCursor` true _returnvalue))

(event `Key|Q`
  (params (Key :type "Key Structure"))
  (bind _returnvalue (`GameplayStatics.GetPlayerController` 0))
  (:`Pressed`
    (bind _asbp_first_person_character (cast `/Game/FirstPerson/Blueprints/BP_FirstPersonCharacter` (`GameplayStatics.GetPlayerCharacter` 0)))
    (`PlayerController.SetViewTargetWithBlend` _returnvalue _asbp_first_person_character 0.5 "VTBlend_Linear" 0.0 false)
    (set `PlayerController.bEnableClickEvents` false _returnvalue)
    (set `PlayerController.bShowMouseCursor` false _returnvalue)))

(event `self.Button.OnClicked`
  (params (TouchedComponent :type "PrimitiveComponent Object Reference") (ButtonPressed :type "Key Structure"))
  (`KismetSystemLibrary.PrintString` "Hello")
  (`/Engine/EditorBlueprintResources/StandardMacros.FlipFlop`
    (:`A`
      (set `self.Desplazamiento` (40.0 10.0 70.0)))
    (:`B`
      (set `self.Desplazamiento` (40.0 10.0 100.0))))
  (`KismetSystemLibrary.MoveComponentTo` (`self.Button`) (`self.Desplazamiento`)))

(fn `UserConstructionScript`)
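; Welding particle Blueprint that moves a Niagara effect along a spline under keyboard control.
; BeginPlay enables input from the first player controller, and holding 5 or 6 sets a forward or backward step that clears on release.
; Each Tick adds that step to an accumulated distance, unscaled by delta time and unclamped, and places the effect at that point on the spline.
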(event `self.ReceiveBeginPlay`
  (`self.EnableInput` (`GameplayStatics.GetPlayerController` 0)))

(event `self.ReceiveTick`
  (params (DeltaSeconds :type "Float (single-precision)"))
  (set `self.Speed` (+ (`self.Speed`) (`self.Acceleration`)))
  (`SceneComponent.K2_SetWorldLocation` (`self.Niagara`) (`SplineComponent.GetLocationAtDistanceAlongSpline` (`self.Spline`) (`self.Speed`) "World") false false))

(event `Key|Five`
  (params (Key :type "Key Structure"))
  (:`Pressed`
    (set `self.Acceleration` 1.0))
  (:`Released`
    (set `self.Acceleration` 0.0 :!label _label)))

(event `Key|Six`
  (params (Key :type "Key Structure"))
  (:`Pressed`
    (set `self.Acceleration` -1.0))
  (:`Released`
    (goto _label)))

(fn `UserConstructionScript`)
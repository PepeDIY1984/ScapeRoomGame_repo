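; BP_Sonidos is an audio demo actor showing 2D and positional sound playback.
; Overlapping its Box plays a one-shot 2D sound.
; BeginPlay enables player input and spawns a persistent music component, immediately stopped, which keys 2 and 3 play and stop.
; Key 1 plays a 3D sound at the Explosion3D actor's location, briefly swapping that static mesh's material as visual feedback.
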(event `self.Box.OnComponentBeginOverlap`
  (params (OverlappedComponent :type "PrimitiveComponent Object Reference") (OtherActor :type "Actor Object Reference") (OtherComp :type "PrimitiveComponent Object Reference") (OtherBodyIndex :type Integer) (bFromSweep :type Boolean) (SweepResult :type "HitResult Structure (by ref)"))
  ; Sonido 2D
  (`GameplayStatics.PlaySound2D` "/Game/BluePrints/009_Media/Sonidos/MS_Sonido2D.MS_Sonido2D" 1.0 1.0 0.0 null null))

(event `Key|Two`
  (params (Key :type "Key Structure"))
  ; Sonido 2D con control de stop y play
  (:`Pressed`
    (`AudioComponent.Play` (stale `self.ReceiveBeginPlay` _returnvalue) 0.0)))

(event `self.ReceiveBeginPlay`
  ; Sonido 2D con control de stop y play
  (`self.EnableInput` (`GameplayStatics.GetPlayerController` 0))
  (bind _returnvalue (`GameplayStatics.SpawnSound2D` "/Game/StarterContent/Audio/Starter_Music_Cue.Starter_Music_Cue" 1.0 1.0 0.0 null false false))
  (`AudioComponent.Stop` _returnvalue :!label _label))

(event `Key|Three`
  (params (Key :type "Key Structure"))
  ; Sonido 2D con control de stop y play
  (:`Pressed`
    (goto _label)))

(event `Key|One`
  (params (Key :type "Key Structure"))
  (bind _explosion3d (`self.explosion3D`))
  ; Sonido 3D al pulsar "1"
  (:`Pressed`
    (bind _asstatic_mesh_actor (cast `StaticMeshActor` _explosion3d))
    (bind _staticmeshcomponent (`StaticMeshActor.StaticMeshComponent` _asstatic_mesh_actor))
    (`PrimitiveComponent.SetMaterial` _staticmeshcomponent 0 "/Engine/VREditor/LaserPointer/LaserPointerMaterial.LaserPointerMaterial")
    (`GameplayStatics.PlaySoundAtLocation` "/Game/BluePrints/009_Media/Sonidos/MS_Sonido3D.MS_Sonido3D" (`self.K2_GetActorLocation` _explosion3d) (struct) 1.0 1.0 0.0 null null null null)
    (`KismetSystemLibrary.Delay` 0.2)
    (`PrimitiveComponent.SetMaterial` _staticmeshcomponent 0 "/Engine/EditorMeshes/ColorCalibrator/M_GreyBall.M_GreyBall")))

(fn `UserConstructionScript`)
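; LineCast is an actor Blueprint that detects DoorLineCast actors in front of it and rotates them.
; Every tick it fires a short Visibility line trace along its forward vector from slightly above its location, with one-frame debug drawing.
; When the hit actor's class is exactly DoorLineCast, it adds a 90-degree local rotation to that actor, repeating on every frame the hit persists.
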(event `self.ReceiveTick`
  (params (DeltaSeconds :type "Float (single-precision)"))
  (bind _returnvalue (+ (`KismetMathLibrary.MakeVector` 0.0 0.0 5.0) (`self.K2_GetActorLocation`)))
  (bind (_outhit _returnvalue_2) (`KismetSystemLibrary.LineTraceSingle` :`Start` _returnvalue :`End` (+ _returnvalue (* (`KismetMathLibrary.GetForwardVector` (`self.K2_GetActorRotation`)) 200.0)) :`TraceChannel` "TraceTypeQuery1" :`DrawDebugType` "ForOneFrame"))
  (if _returnvalue_2
    (bind (_bblockinghit _binitialoverlap _time _distance _location _impactpoint _normal _impactnormal _physmat _hitactor) (`GameplayStatics.BreakHitResult` _outhit))
    (if (== (`GameplayStatics.GetObjectClass` _hitactor) "/Game/BluePrints/UD1_2_LineTracer/DoorLineCast.DoorLineCast_C")
      (`self.K2_AddActorLocalRotation` _hitactor (struct :`Yaw` 90.0) false false))))

(fn `UserConstructionScript`)
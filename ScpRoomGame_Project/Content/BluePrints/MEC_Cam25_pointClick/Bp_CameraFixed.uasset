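; Fixed-camera point-and-click puzzle panel: entering TriggerArea blends the view to this actor, shows the cursor and freezes the player, and Q restores both.
; Clicks drive a toggling slider, a bar that follows the cursor's hit height within clamped limits, and four buttons that record a combination.
; A check button compares it digit by digit with the correct array, which the lever click fills, showing green or red and resetting on mismatch.
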(event `self.ReceiveBeginPlay`
  ; Activar input
  (`self.EnableInput` (`GameplayStatics.GetPlayerController` 0)))

(event `self.TriggerArea.OnComponentBeginOverlap`
  (params (OverlappedComponent :type "PrimitiveComponent Object Reference") (OtherActor :type "Actor Object Reference") (OtherComp :type "PrimitiveComponent Object Reference") (OtherBodyIndex :type Integer) (bFromSweep :type Boolean) (SweepResult :type "HitResult Structure (by ref)"))
  (bind _returnvalue (`GameplayStatics.GetPlayerController` 0))
  ; Al entrar en el trigger cambiar la camara del Player a la propia de este blueprint "self", activar eventos de click y mostrar el cursor
  (`PlayerController.SetViewTargetWithBlend` _returnvalue self 0.5 "VTBlend_Linear" 0.0 false)
  (set `PlayerController.bEnableClickEvents` true _returnvalue)
  (set `PlayerController.bShowMouseCursor` true _returnvalue)
  (set `PlayerController.bEnableMouseOverEvents` true _returnvalue)
  ;[0.02189 0.0219 0.15 0.5] Activar o desactivar movimiento del Player cuando tiene la camara fija
  (`CharacterMovementComponent.DisableMovement` (`Character.CharacterMovement` (`GameplayStatics.GetPlayerCharacter` 0))))

(event `Key|Q`
  (params (Key :type "Key Structure"))
  (bind _returnvalue (`GameplayStatics.GetPlayerController` 0))
  ; Si se pulsa Q volver a la camara del Player y su movimiento
  (:`Pressed`
    (bind _asbp_first_person_character (cast `/Game/FirstPerson/Blueprints/BP_FirstPersonCharacter` (`GameplayStatics.GetPlayerCharacter` 0)))
    (`PlayerController.SetViewTargetWithBlend` _returnvalue _asbp_first_person_character 0.5 "VTBlend_Linear" 0.0 false)
    (set `PlayerController.bEnableClickEvents` false _returnvalue)
    (set `PlayerController.bShowMouseCursor` false _returnvalue)
    ;[0.02189 0.0219 0.15 0.5] Activar o desactivar movimiento del Player cuando tiene la camara fija
    (`CharacterMovementComponent.SetMovementMode` (`Character.CharacterMovement` (`GameplayStatics.GetPlayerCharacter` 0)) "MOVE_Walking" 0)))

(event `self.ButtonSlider.OnClicked`
  (params (TouchedComponent :type "PrimitiveComponent Object Reference") (ButtonPressed :type "Key Structure"))
  ; Button2:  Cambio de posición
  (`/Engine/EditorBlueprintResources/StandardMacros.FlipFlop`
    (:`A`
      (set `self.desplazamiento` -10.0))
    (:`B`
      (set `self.desplazamiento` 10.0)))
  (`KismetSystemLibrary.MoveComponentTo` (`self.ButtonSlider`) (`KismetMathLibrary.MakeVector` 0.0 0.0 (`self.desplazamiento`)) (struct) true true 1.0))

(event `self.ReceiveTick`
  (params (DeltaSeconds :type "Float (single-precision)"))
  ;[0.1445 0.15 0.142 0.5] SISTEMA DE BARRAS DE ARRASTRE
  ;; Actualizar la posición de la barra
  (if (`self.IsSelected`)
    (`SceneComponent.K2_SetWorldLocation` (`self.Barra`) (`KismetMathLibrary.MakeVector` (.x (`SceneComponent.K2_GetComponentLocation` (`self.Barra`))) (.y (`SceneComponent.K2_GetComponentLocation` (`self.Barra`))) (`KismetMathLibrary.FClamp` (.z (`.ImpactPoint` (`GameplayStatics.BreakHitResult` (`PlayerController.GetHitResultUnderCursorByChannel` (`GameplayStatics.GetPlayerController` 0) "TraceTypeQuery1" true)))) 130.0 164.0)) true false)
    (if (> (.z (`SceneComponent.K2_GetComponentLocation` (`self.Barra`))) 150.0)
      (`KismetSystemLibrary.PrintString` "Peligro!!"))))

(event `self.Barra.OnBeginCursorOver`
  (params (TouchedComponent :type "PrimitiveComponent Object Reference"))
  ;[0.1445 0.15 0.142 0.5] SISTEMA DE BARRAS DE ARRASTRE
  ;; Seleccionar la barra
)

(event `self.Barra.OnClicked`
  (params (TouchedComponent :type "PrimitiveComponent Object Reference") (ButtonPressed :type "Key Structure"))
  ;[0.1445 0.15 0.142 0.5] SISTEMA DE BARRAS DE ARRASTRE
  ;; Seleccionar la barra
  (set `self.IsSelected` true)
  (`PrimitiveComponent.SetMaterial` (`self.Barra`) 0 "/Game/LevelPrototyping/Materials/MI_Solid_Blue.MI_Solid_Blue"))

(event `self.Fondo.OnClicked`
  (params (TouchedComponent :type "PrimitiveComponent Object Reference") (ButtonPressed :type "Key Structure"))
  ;[0.1445 0.15 0.142 0.5] SISTEMA DE BARRAS DE ARRASTRE
  ;; Seleccionar la barra
  (set `self.IsSelected` false)
  (`PrimitiveComponent.SetMaterial` (`self.Barra`) 0 "/Engine/EditorMeshes/ColorCalibrator/M_GreyBall.M_GreyBall"))

(event `self.Button004.OnClicked`
  (params (TouchedComponent :type "PrimitiveComponent Object Reference") (ButtonPressed :type "Key Structure"))
  ; Button1: Cambio de material
  (`PrimitiveComponent.SetMaterial` (`self.Button004`) 0 "/Engine/EngineDebugMaterials/VertexColorViewMode_BlueOnly.VertexColorViewMode_BlueOnly")
  (`KismetArrayLibrary.Array_Add` (`self.combinacion`) 4)
  (`KismetSystemLibrary.PrintString` "4"))

(event `self.Button001.OnClicked`
  (params (TouchedComponent :type "PrimitiveComponent Object Reference") (ButtonPressed :type "Key Structure"))
  ; Button1: Cambio de material
  (`PrimitiveComponent.SetMaterial` (`self.Button001`) 0 "/Engine/EngineDebugMaterials/VertexColorViewMode_BlueOnly.VertexColorViewMode_BlueOnly")
  (`KismetArrayLibrary.Array_Add` (`self.combinacion`) 1)
  (`KismetSystemLibrary.PrintString` "1"))

(event `self.Button003.OnClicked`
  (params (TouchedComponent :type "PrimitiveComponent Object Reference") (ButtonPressed :type "Key Structure"))
  ; Button1: Cambio de material
  (`PrimitiveComponent.SetMaterial` (`self.Button003`) 0 "/Engine/EngineDebugMaterials/VertexColorViewMode_BlueOnly.VertexColorViewMode_BlueOnly")
  (`KismetArrayLibrary.Array_Add` (`self.combinacion`) 3)
  (`KismetSystemLibrary.PrintString` "3"))

(event `self.Button002.OnClicked`
  (params (TouchedComponent :type "PrimitiveComponent Object Reference") (ButtonPressed :type "Key Structure"))
  ; Button1: Cambio de material
  (`PrimitiveComponent.SetMaterial` (`self.Button002`) 0 "/Engine/EngineDebugMaterials/VertexColorViewMode_BlueOnly.VertexColorViewMode_BlueOnly")
  (`KismetArrayLibrary.Array_Add` (`self.combinacion`) 2)
  (`KismetSystemLibrary.PrintString` "2"))

(event `self.Palanca.OnClicked`
  (params (TouchedComponent :type "PrimitiveComponent Object Reference") (ButtonPressed :type "Key Structure"))
  (bind _combinacioncorrecta (`self.combinacionCorrecta`))
  ; Definir la array de la combinación correcta inicialmente en el BP o en la pestaña de Details
  (`KismetArrayLibrary.Array_Add` _combinacioncorrecta 1)
  (`KismetArrayLibrary.Array_Add` _combinacioncorrecta 2)
  (`KismetArrayLibrary.Array_Add` _combinacioncorrecta 3)
  (`KismetArrayLibrary.Array_Add` _combinacioncorrecta 4))

(event `self.ButtonComprobar.OnClicked`
  (params (TouchedComponent :type "PrimitiveComponent Object Reference") (ButtonPressed :type "Key Structure"))
  ; Recorrer las 2 arrays e ir comprobando cada uno de los digitos
  (for (_array_element _array_index) (`self.combinacionCorrecta`)
    (bind _output (`|GetArrayItem` (`self.combinacion`) _array_index))
    ; Definir mensajes si son o no iguales las cifras
    (if (== _array_element _output)
      (set `self.mensaje` " son iguales")
      ; Si son iguales cambiar el color del botón de comprobación a verde
      (`PrimitiveComponent.SetMaterial` (`self.ButtonComprobar`) 0 "/Engine/EngineDebugMaterials/VertexColorViewMode_GreenOnly.VertexColorViewMode_GreenOnly")
      (bind _returnvalue (`KismetStringLibrary.Concat_StrStr` (`KismetStringLibrary.Conv_IntToString` _output) "  VS  " (`KismetStringLibrary.Conv_IntToString` _array_element) (`self.mensaje`)))
      (`KismetSystemLibrary.PrintString` _returnvalue true true (struct :`G` 0.66 :`B` 1.0 :`A` 1.0) 5.0)
      (else
        (set `self.mensaje` " NO son iguales")
        ; Si no son iguales, cambiar los botones a gris, y vaciar la variable combinacion para poder volver a empezar
        (`PrimitiveComponent.SetMaterial` (`self.ButtonComprobar`) 0 "/Engine/EngineDebugMaterials/VertexColorViewMode_RedOnly.VertexColorViewMode_RedOnly")
        (`PrimitiveComponent.SetMaterial` (`self.Button001`) 0 "/Engine/EditorMeshes/ColorCalibrator/M_GreyBall.M_GreyBall")
        (`PrimitiveComponent.SetMaterial` (`self.Button002`) 0 "/Engine/EditorMeshes/ColorCalibrator/M_GreyBall.M_GreyBall")
        (`PrimitiveComponent.SetMaterial` (`self.Button003`) 0 "/Engine/EditorMeshes/ColorCalibrator/M_GreyBall.M_GreyBall")
        (`PrimitiveComponent.SetMaterial` (`self.Button004`) 0 "/Engine/EditorMeshes/ColorCalibrator/M_GreyBall.M_GreyBall")
        (`KismetSystemLibrary.PrintString` _returnvalue true true (struct :`G` 0.66 :`B` 1.0 :`A` 1.0) 5.0)
        (`KismetSystemLibrary.Delay` 0.2)
        (`KismetArrayLibrary.Array_Clear` (`self.combinacion`))
        (`PrimitiveComponent.SetMaterial` (`self.ButtonComprobar`) 0 "/Engine/EditorMeshes/ColorCalibrator/M_GreyBall.M_GreyBall")))))

(fn `UserConstructionScript`)
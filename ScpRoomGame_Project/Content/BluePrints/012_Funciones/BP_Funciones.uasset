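; BP_Funciones is an example actor demonstrating Blueprint functions, using counters shown on TextRender components.
; It enables player input on BeginPlay, and a left click calls FuncionContadorParametros with a text component and counter.
; That function increments the counter, displays it up to five, then returns true.
; Unwired examples show inline counting, the parameterless FuncionContador, and chaining two counters through the returned boolean.
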(event `self.ReceiveBeginPlay`
  ; Activar inputs
  (`self.EnableInput` (`GameplayStatics.GetPlayerController` 0)))

(event `Key|LeftMouseButton`
  (params (Key :type "Key Structure"))
  ; Funciones con parámetros
  (:`Pressed`
    (`self.FuncionContadorParametros` (`self.TextRender`) (`self.contador`))))

(fn `FuncionContador`
  (bind _result (`/Engine/EditorBlueprintResources/StandardMacros.IncrementInt` (`self.contador`))
    (:`  `
      (`TextRenderComponent.K2_SetText` (`self.TextRender`) (`KismetTextLibrary.Conv_IntToText` _result)))))

(fn `FuncionContadorParametros`
  (params (Texto3D :type "TextRenderComponent Object Reference") (Contador :type "Integer (by ref)"))
  (returns (ActivarSiguiente :type Boolean))
  (locals (contadorLocal :type Integer))
  (bind _result (`/Engine/EditorBlueprintResources/StandardMacros.IncrementInt` Contador)
    (:`  `
      (if (<= _result 5)
        (`TextRenderComponent.K2_SetText` Texto3D (`KismetTextLibrary.Conv_IntToText` _result))
        (elif true
          (return true))))))

(fn `UserConstructionScript`)
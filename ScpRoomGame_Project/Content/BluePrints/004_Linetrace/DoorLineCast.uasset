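; DoorLineCast is a door Blueprint that swings open when its StartOpenDoor event is called.
; The event plays a timeline whose AnimPuerta track lerps between closed and open values to set the Arrow component's relative yaw, animating the door procedurally.
; Two disconnected alternatives remain in the graph: playing a baked Linetrace Level Sequence and snapping the Arrow to a fixed rotation without animation.
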(event `/Game/BluePrints/004_Linetrace/BPI_OpenDoor.StartOpenDoor`
  ; Animación procedural
  (bind (_direction _animpuerta) (`Timeline|Timeline_0`)
    (:`Update`
      (`SceneComponent.K2_SetRelativeRotation` (`self.Arrow`) (`KismetMathLibrary.MakeRotator` 0.0 0.0 (`KismetMathLibrary.Lerp` (`self.PuertaCerrada`) (`self.PuertaAbierta`) _animpuerta)) false false))))

(fn `UserConstructionScript`)
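; LineCast is an actor Blueprint that detects door actors in front of it and rotates them.
; Every Tick it fires a short debug-drawn Visibility line trace along its forward vector, starting slightly above its origin.
; When the hit actor's class is exactly DoorLineCast, it adds a 90-degree local rotation to that actor.
; No guard limits this, so the rotation repeats every frame the trace keeps hitting.
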(event `self.ReceiveTick`
  (params (DeltaSeconds :type "Float (single-precision)"))
  (bind _returnvalue (+ (`KismetMathLibrary.MakeVector` 0.0 0.0 5.0) (`self.K2_GetActorLocation`)))
  ; Crear un raycast desde un actor
  ;; Crear rayo a cada frame y detectar colision
  (bind _outhit (`KismetSystemLibrary.LineTraceSingle` :`Start` _returnvalue :`End` (+ _returnvalue (* (`KismetMathLibrary.GetForwardVector` (`self.K2_GetActorRotation`)) 200.0)) :`TraceChannel` "TraceTypeQuery1" :`DrawDebugType` "ForOneFrame"))
  (bind (_bblockinghit _binitialoverlap _time _distance _location _impactpoint _normal _impactnormal _physmat _hitactor) (`GameplayStatics.BreakHitResult` _outhit))
  ;; Si la colision es con un actor de clase Door Line Cast girar el actor colisionado 90º
  (if (== (`GameplayStatics.GetObjectClass` _hitactor) "/Game/BluePrints/006_Inputs/DoorLineCast.DoorLineCast_C")
    (`self.K2_AddActorLocalRotation` _hitactor (struct :`Yaw` -90.0) false false)))

(fn `UserConstructionScript`)
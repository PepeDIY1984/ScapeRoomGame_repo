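; BP_areaNado is a swim volume that lets the first-person character dive and move vertically inside a box trigger.
; On overlap it fakes swimming by switching the character to Flying movement, stopping its momentum and lowering fly speed; leaving restores Walking and normal speed.
; It enables input on itself at BeginPlay and feeds the SwimUp axis into world-Z movement on player 0, without checking whether that character is inside the box.
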(event `self.ReceiveBeginPlay`
  ; Activar inputs
  (`self.EnableInput` (`GameplayStatics.GetPlayerController` 0)))

(event `InputAxis|SwimUp`
  (params (AxisValue :type "Float (single-precision)"))
  ; Inputs tipo eje con la q y la e
  (`Pawn.AddMovementInput` (`GameplayStatics.GetPlayerCharacter` 0) (0.0 0.0 1.0) AxisValue false))

(event `self.Box.OnComponentBeginOverlap`
  (params (OverlappedComponent :type "PrimitiveComponent Object Reference") (OtherActor :type "Actor Object Reference") (OtherComp :type "PrimitiveComponent Object Reference") (OtherBodyIndex :type Integer) (bFromSweep :type Boolean) (SweepResult :type "HitResult Structure (by ref)"))
  ; Cambiar a modo buceo/vuelo al entrar y frenar la velocidad
  (bind _asbp_first_person_character (cast `/Game/FirstPerson/Blueprints/BP_FirstPersonCharacter` OtherActor))
  (bind _charactermovement (`Character.CharacterMovement` _asbp_first_person_character))
  (`CharacterMovementComponent.SetMovementMode` _charactermovement "MOVE_Flying" 0)
  (`MovementComponent.StopMovementImmediately` _charactermovement)
  (set `CharacterMovementComponent.MaxFlySpeed` 150.0 _charactermovement))

(event `self.Box.OnComponentEndOverlap`
  (params (OverlappedComponent :type "PrimitiveComponent Object Reference") (OtherActor :type "Actor Object Reference") (OtherComp :type "PrimitiveComponent Object Reference") (OtherBodyIndex :type Integer))
  ; Cambiar a modo caminar al salir del trigger
  (bind _asbp_first_person_character (cast `/Game/FirstPerson/Blueprints/BP_FirstPersonCharacter` OtherActor))
  (bind _charactermovement (`Character.CharacterMovement` _asbp_first_person_character))
  (`CharacterMovementComponent.SetMovementMode` _charactermovement "MOVE_Walking" 0)
  (set `CharacterMovementComponent.MaxWalkSpeed` 600.0 _charactermovement))

(fn `UserConstructionScript`)
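; BP_WidgetManager creates the WB_Mainmenu widget and toggles one of its images through a box trigger.
; On BeginPlay it stores the widget, adds it to the viewport and hides Image0.
; Any overlap with the Box shows the image, increments the widget's Numero counter and prints a greeting.
; Ending the overlap hides the image again, with no check on the overlapping actor.
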(event `self.ReceiveBeginPlay`
  (bind _returnvalue (`|CreateWidget` "/Game/BluePrints/004_Widgets/WB_Mainmenu.WB_Mainmenu_C"))
  (set `self.WB_MainMenu` _returnvalue)
  (`UserWidget.AddToViewport` _returnvalue 0)
  (set `Widget.Visibility` "Hidden" (`/Game/BluePrints/004_Widgets/WB_Mainmenu.Image_0` _returnvalue)))

(event `self.Box.OnComponentBeginOverlap`
  (params (OverlappedComponent :type "PrimitiveComponent Object Reference") (OtherActor :type "Actor Object Reference") (OtherComp :type "PrimitiveComponent Object Reference") (OtherBodyIndex :type Integer) (bFromSweep :type Boolean) (SweepResult :type "HitResult Structure (by ref)"))
  (set `Widget.Visibility` "Visible" (`/Game/BluePrints/004_Widgets/WB_Mainmenu.Image_0` (stale `self.ReceiveBeginPlay` _returnvalue)))
  (`/Engine/EditorBlueprintResources/StandardMacros.IncrementInt` (`/Game/BluePrints/004_Widgets/WB_Mainmenu.numero` (stale `self.ReceiveBeginPlay` _returnvalue))
    (:`  `
      (`KismetSystemLibrary.PrintString` "Hello"))))

(event `self.Box.OnComponentEndOverlap`
  (params (OverlappedComponent :type "PrimitiveComponent Object Reference") (OtherActor :type "Actor Object Reference") (OtherComp :type "PrimitiveComponent Object Reference") (OtherBodyIndex :type Integer))
  (set `Widget.Visibility` "Hidden" (`/Game/BluePrints/004_Widgets/WB_Mainmenu.Image_0` (stale `self.ReceiveBeginPlay` _returnvalue))))

(fn `UserConstructionScript`)
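; Door trigger actor that shows an open-door widget while something overlaps its box and swings the door open on F.
; At BeginPlay it enables input and creates a menu widget plus the hidden door prompt; each overlap increments the menu's counter.
; F plays a Timeline that lerps the door yaw to -90 degrees, and Q toggles the mouse cursor.
; Unconnected alternatives open the door via a Level Sequence or instant rotation.
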(event `self.ReceiveBeginPlay`
  ; Activar inputs en este script
  (`self.EnableInput` (`GameplayStatics.GetPlayerController` 0))
  ; Crear widget de Menu
  (bind _returnvalue (`|CreateWidget` "/Game/BluePrints/004_Widgets/AperturaPuerta/GUI_Menu.GUI_Menu_C"))
  (`UserWidget.AddToViewport` _returnvalue 0)
  ; Crear Widget de apertura de puerta
  (bind _returnvalue_2 (`|CreateWidget` "/Game/BluePrints/004_Widgets/AperturaPuerta/GUI_OpenDoor.GUI_OpenDoor_C"))
  (bind _output_get (set `self.GUI` _returnvalue_2))
  (`UserWidget.AddToViewport` _output_get 0)
  (`Widget.SetVisibility` (`self.GUI`) "Hidden"))

(event `self.Box.OnComponentBeginOverlap`
  (params (OverlappedComponent :type "PrimitiveComponent Object Reference") (OtherActor :type "Actor Object Reference") (OtherComp :type "PrimitiveComponent Object Reference") (OtherBodyIndex :type Integer) (bFromSweep :type Boolean) (SweepResult :type "HitResult Structure (by ref)"))
  ; Cuando se entra en la zona de trigger mostrar widget de apertura y contar las veces que se ha accedido al área de trigger
  (`Widget.SetVisibility` (`self.GUI`) "Visible")
  (bind _result (`/Engine/EditorBlueprintResources/StandardMacros.IncrementInt` (`/Game/BluePrints/004_Widgets/AperturaPuerta/GUI_Menu.numero` (stale `self.ReceiveBeginPlay` _returnvalue)))
    (:`  `
      (set `/Game/BluePrints/004_Widgets/AperturaPuerta/GUI_Menu.numero` _result (stale `self.ReceiveBeginPlay` _returnvalue)))))

(event `Key|Q`
  (params (Key :type "Key Structure"))
  (bind _returnvalue (`GameplayStatics.GetPlayerController` 0))
  ; Mostrar/ocultar el cursor al pulsar "q"
  (:`Pressed`
    (`/Engine/EditorBlueprintResources/StandardMacros.FlipFlop`
      (:`A`
        (set `PlayerController.bShowMouseCursor` true _returnvalue))
      (:`B`
        (set `PlayerController.bShowMouseCursor` false _returnvalue)))))

(event `self.Box.OnComponentEndOverlap`
  (params (OverlappedComponent :type "PrimitiveComponent Object Reference") (OtherActor :type "Actor Object Reference") (OtherComp :type "PrimitiveComponent Object Reference") (OtherBodyIndex :type Integer))
  ; Cuando se entra en la zona de trigger mostrar widget de apertura y contar las veces que se ha accedido al área de trigger
  (`Widget.SetVisibility` (`self.GUI`) "Hidden"))

(event `Key|F`
  (params (Key :type "Key Structure"))
  ; Distintos modos de apertura de puerta
  (:`Pressed`
    ;; Animación procedural
    (bind (_direction _animpuerta) (`Timeline|Timeline`)
      (:`Update`
        (`SceneComponent.K2_SetRelativeRotation` (`self.Door`) (`KismetMathLibrary.MakeRotator` 0.0 0.0 (`KismetMathLibrary.Lerp` 0.0 -90.0 _animpuerta)) false false)))))

(fn `UserConstructionScript`)
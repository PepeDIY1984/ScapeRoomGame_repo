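; BP_Translate is a movement actor that shuttles back and forth along the world X axis between two hard-coded bounds.
; BeginPlay sets the starting Speed, and each Tick offsets the actor's location by that amount without sweep.
; When X lies outside the bounds, Speed flips sign before the move.
; The step is not scaled by delta time, so travel speed depends on frame rate.
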(event `self.ReceiveBeginPlay`
  ; Inicializar velocidad
  (set `self.Speed` 1.0))

(event `self.ReceiveTick`
  (params (DeltaSeconds :type "Float (single-precision)"))
  (bind _x (.x (`self.K2_GetActorLocation`)))
  ; Bucle principal, si la coordenada x esta entre 200 y 600 se mueve, sino invierte la velocidad multiplicandola por -1
  (if (or (< _x 200.0) (> _x 600.0))
    (set `self.Speed` (* (`self.Speed`) -1.0)))
  (`self.K2_SetActorLocation` (+ (`self.K2_GetActorLocation`) (`KismetMathLibrary.MakeVector` (`self.Speed`)))))

(fn `UserConstructionScript`)
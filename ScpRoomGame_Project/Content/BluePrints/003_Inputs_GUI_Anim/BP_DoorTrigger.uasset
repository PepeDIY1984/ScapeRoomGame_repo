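; BP_DoorTrigger is a door actor with a trigger box that lets the player open the door with E.
; On BeginPlay it enables input and creates a menu widget and a hidden open-door prompt.
; Overlapping the box shows or hides the prompt and increments the menu's entry counter.
; E plays a Timeline rotating the door's yaw; Sequencer, instant-rotation and cursor-toggle alternatives are left disconnected.
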(event `self.ReceiveBeginPlay`
  ; Activar inputs en este script
  (`self.EnableInput` (`GameplayStatics.GetPlayerController` 0))
  ; Crear widget de Menu
  (bind _returnvalue (`|CreateWidget` "/Game/BluePrints/003_Inputs_GUI_Anim/GUI_Menu.GUI_Menu_C"))
  (`UserWidget.AddToViewport` _returnvalue 0)
  ; Crear Widget de apertura de puerta
  (bind _returnvalue_2 (`|CreateWidget` "/Game/BluePrints/003_Inputs_GUI_Anim/GUI_OpenDoor.GUI_OpenDoor_C"))
  (bind _output_get (set `self.GUI` _returnvalue_2))
  (`UserWidget.AddToViewport` _output_get 0)
  (`Widget.SetVisibility` (`self.GUI`) "Hidden"))

(event `self.Box.OnComponentBeginOverlap`
  (params (OverlappedComponent :type "PrimitiveComponent Object Reference") (OtherActor :type "Actor Object Reference") (OtherComp :type "PrimitiveComponent Object Reference") (OtherBodyIndex :type Integer) (bFromSweep :type Boolean) (SweepResult :type "HitResult Structure (by ref)"))
  ; Cuando se entra en la zona de trigger mostrar widget de apertura y contar las veces que se ha accedido al área de trigger
  (`Widget.SetVisibility` (`self.GUI`) "Visible")
  (bind _result (`/Engine/EditorBlueprintResources/StandardMacros.IncrementInt` (`/Game/BluePrints/003_Inputs_GUI_Anim/GUI_Menu.numero_` (stale `self.ReceiveBeginPlay` _returnvalue)))
    (:`  `
      (set `/Game/BluePrints/003_Inputs_GUI_Anim/GUI_Menu.numero_` _result (stale `self.ReceiveBeginPlay` _returnvalue)))))

(event `Key|Q`
  (params (Key :type "Key Structure"))
  ; Mostrar/ocultar el cursor al pulsar "q"
)

(event `self.Box.OnComponentEndOverlap`
  (params (OverlappedComponent :type "PrimitiveComponent Object Reference") (OtherActor :type "Actor Object Reference") (OtherComp :type "PrimitiveComponent Object Reference") (OtherBodyIndex :type Integer))
  ; Cuando se entra en la zona de trigger mostrar widget de apertura y contar las veces que se ha accedido al área de trigger
  (`Widget.SetVisibility` (`self.GUI`) "Hidden"))

(event `Key|E`
  (params (Key :type "Key Structure"))
  ; Distintos modos de apertura de puerta
  ;; Animación procedural
  (:`Pressed`
    (bind (_direction _animpuerta _animpuerta2) (`Timeline|Timeline`)
      (:`Update`
        (`KismetSystemLibrary.PrintString` (`KismetStringLibrary.Conv_DoubleToString` _animpuerta2))
        (`SceneComponent.K2_SetRelativeRotation` (`self.Door`) (`KismetMathLibrary.MakeRotator` 0.0 0.0 _animpuerta2) false false)))))

(fn `UserConstructionScript`)
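; Interactive cylinder for a scale-timing mechanic: its height oscillates and the player tries to stop it within a target range.
; Tick grows and shrinks the root's Z scale, reversing the speed at the limits.
; The E key toggles stopping through a FlipFlop; stopping swaps in a success material, or a failure material plus an error message, depending on scale.
; Resuming restores the glass material, and PararCilindro is an empty event.
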(event `self.ReceiveBeginPlay`
  ;[0.15 0.001563 0.004936 0.5] Activar inputs de teclado y asignar material inicial al cilindro
  (`self.EnableInput` (`GameplayStatics.GetPlayerController` 0))
  (`PrimitiveComponent.CreateDynamicMaterialInstance` (`self.Cylinder`) 0 "/Game/StarterContent/Materials/M_Glass.M_Glass" "None"))

(event `self.ReceiveTick`
  (params (DeltaSeconds :type "Float (single-precision)"))
  (bind _scalez (`self.scaleZ`))
  ;[0.07707 0.15 0.05556 0.5] Aumentar y disminuir la escala en el eje z entre 2 coordenadas específicas
  ;; Variar la escalaZ solo si no esta parado
  (if (not (`self.bIsStopped`))
    (bind _output_get (set `self.scaleZ` (+ (`self.scaleZ`) (`self.ScaleSpeed`))))
    ;; Si la escalaZ está entre estos 2 valores
    (if (and (< _scalez 3.0) (> _scalez 0.0))
      (`SceneComponent.SetWorldScale3D` (`self.DefaultSceneRoot`) (`KismetMathLibrary.MakeVector` 1.0 1.0 _output_get))
      (else
        ;; Invertir dirección del incremento de la escalaZ
        (set `self.ScaleSpeed` (* (`self.ScaleSpeed`) -1.0))))))

(event `Key|E`
  (params (Key :type "Key Structure"))
  (bind _scalez (`self.scaleZ`))
  ;[0.04614 0.07211 0.15 0.5] Si se pulsa la "e" y no está parada la variación de la escalaZ: asignar material glass al cilindro
  (:`Pressed`
    (`/Engine/EditorBlueprintResources/StandardMacros.FlipFlop`
      (:`A`
        (set `self.bIsStopped` true)
        ;[0.04614 0.07211 0.15 0.5] Si el cilindro se para comprobar que esta entre las coordenadas 2 y 1.2
        (if (and (< _scalez 2.0) (> _scalez 1.2))
          ;[0.04614 0.07211 0.15 0.5] Si está entre las coordenadas asignar material "verde"
          (`PrimitiveComponent.CreateDynamicMaterialInstance` (`self.Cylinder`) 0 "/Engine/ArtTools/RenderToTexture/Materials/M_RadiusDebugTranslucent.M_RadiusDebugTransLucent" "None")
          (else
            ;[0.04614 0.07211 0.15 0.5] Si no está entre las coordenadas asignar material "rojo" y mostrar un mensaje de error
            (`KismetSystemLibrary.PrintString` "ERROR" true true (struct :`R` 1.0 :`B` 0.207749 :`A` 1.0))
            (`PrimitiveComponent.CreateDynamicMaterialInstance` (`self.Cylinder`) 0 "/Engine/VREditor/LaserPointer/TranslucentLaserPointerMaterialInst.TranslucentLaserPointerMaterialInst" "None"))))
      (:`B`
        (set `self.bIsStopped` false)
        (`PrimitiveComponent.CreateDynamicMaterialInstance` (`self.Cylinder`) 0 "/Game/StarterContent/Materials/M_Glass.M_Glass" "None")))))

(event `self.PararCilindro`)

(fn `UserConstructionScript`)
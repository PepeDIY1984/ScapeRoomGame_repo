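; Cylinder timing puzzle: three bar scales oscillate in Z, and clickable buttons freeze them.
; Tick steps each scale; the third branch mistakenly drives Arrow002 and negates its scale instead of speed.
; Buttons 1 and 2 toggle stop/resume via FlipFlop; stopping within range changes their material and the next button's, without gating clicks.
; Button 3 only stops its scale; BeginPlay enables mouse clicks, and the by-ref CambioEscala refactor is unused.
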(event `self.ReceiveBeginPlay`
  (bind _returnvalue (`GameplayStatics.GetPlayerController` 0))
  (`PrimitiveComponent.SetMaterial` (`self.Cylinder001`) 0 "/Game/BluePrints/MEC_cambioEscala/M_Glass_Inst.M_Glass_Inst")
  (`PrimitiveComponent.SetMaterial` (`self.Button001`) 0 "/Engine/VREditor/LaserPointer/LaserPointerMaterial.LaserPointerMaterial")
  ; Activar onclick
  (set `PlayerController.bEnableClickEvents` true _returnvalue)
  (set `PlayerController.bShowMouseCursor` true _returnvalue)
  (set `PlayerController.bEnableMouseOverEvents` true _returnvalue))

(event `self.ReceiveTick`
  (params (DeltaSeconds :type "Float (single-precision)"))
  (bind _scalez003 (`self.scaleZ003`))
  (bind _scalez001 (`self.scaleZ001`))
  (bind _scalez002 (`self.scaleZ002`))
  (`|ExecutionSequence`
    (:`then_0`
      ; Version para 1 barra
      (bind _output_get (set `self.scaleZ001` (+ (`self.scaleZ001`) (`self.scaleSpeed001`))))
      ;; Si la escalaZ está entre estos 2 valores
      (if (and (< _scalez001 3.0) (> _scalez001 0.0))
        (`SceneComponent.SetWorldScale3D` (`self.Arrow001`) (`KismetMathLibrary.MakeVector` 1.0 1.0 _output_get))
        (else
          ;; Invertir dirección del incremento de la escalaZ
          (set `self.scaleSpeed001` (* (`self.scaleSpeed001`) -1.0)))))
    (:`then_1`
      ; Versión para  barra 002
      (bind _output_get_2 (set `self.scaleZ002` (+ (`self.scaleZ002`) (`self.scaleSpeed002`))))
      ;; Si la escalaZ está entre estos 2 valores
      (if (and (< _scalez002 3.0) (> _scalez002 0.0))
        (`SceneComponent.SetWorldScale3D` (`self.Arrow002`) (`KismetMathLibrary.MakeVector` 1.0 1.0 _output_get_2))
        (else
          ;; Invertir dirección del incremento de la escalaZ
          (set `self.scaleSpeed002` (* (`self.scaleSpeed002`) -1.0)))))
    (:`then_2`
      ; Versión para  barra 003
      (bind _output_get_3 (set `self.scaleZ003` (+ (`self.scaleZ003`) (`self.scaleSpeed003`))))
      ;; Si la escalaZ está entre estos 2 valores
      (if (and (< _scalez003 3.0) (> _scalez003 0.0))
        (`SceneComponent.SetWorldScale3D` (`self.Arrow002`) (`KismetMathLibrary.MakeVector` 1.0 1.0 _output_get_3))
        (else
          ;; Invertir dirección del incremento de la escalaZ
          (set `self.scaleZ003` (* (`self.scaleZ003`) -1.0)))))))

(event `self.Button001.OnClicked`
  (params (TouchedComponent :type "PrimitiveComponent Object Reference") (ButtonPressed :type "Key Structure"))
  (bind _scalez001 (`self.scaleZ001`))
  ; Si se pulsa el botón y el cilindro tiene la escala correcta, se ilumina en verde el botón y se activa el siguiente
  (`/Engine/EditorBlueprintResources/StandardMacros.FlipFlop`
    (:`A`
      (set `self.scaleSpeed001` 0.0)
      (if (and (< _scalez001 2.0) (> _scalez001 0.0))
        (`PrimitiveComponent.SetMaterial` (`self.Button001`) 0 "/Engine/VREditor/LaserPointer/LaserPointerMaterial_Inst.LaserPointerMaterial_Inst")
        (`PrimitiveComponent.SetMaterial` (`self.Button002`) 0 "/Engine/VREditor/LaserPointer/LaserPointerMaterialInst.LaserPointerMaterialInst")))
    (:`B`
      (set `self.scaleSpeed001` 0.01))))

(event `self.Button002.OnClicked`
  (params (TouchedComponent :type "PrimitiveComponent Object Reference") (ButtonPressed :type "Key Structure"))
  (bind _scalez002 (`self.scaleZ002`))
  (`/Engine/EditorBlueprintResources/StandardMacros.FlipFlop`
    (:`A`
      (set `self.scaleSpeed002` 0.0)
      (if (and (< _scalez002 2.0) (> _scalez002 0.0))
        (`PrimitiveComponent.SetMaterial` (`self.Button002`) 0 "/Engine/VREditor/LaserPointer/LaserPointerMaterial_Inst.LaserPointerMaterial_Inst")
        (`PrimitiveComponent.SetMaterial` (`self.Button003`) 0 "/Engine/VREditor/LaserPointer/LaserPointerMaterialInst.LaserPointerMaterialInst")))
    (:`B`
      (set `self.scaleSpeed002` 0.024))))

(event `self.Button003.OnClicked`
  (params (TouchedComponent :type "PrimitiveComponent Object Reference") (ButtonPressed :type "Key Structure"))
  (set `self.scaleSpeed003` 0.0))

(fn `CambioEscala`
  (params (ScaleZ :type "Float (double-precision) (by ref)") (ScaleSpped :type "Float (double-precision) (by ref)") (Arrow :type "ArrowComponent Object Reference"))
  ; Escala z aumentando continuamente
  (`|VariableSetRef` ScaleZ (+ ScaleZ ScaleSpped))
  ; Comprobar si la escala está entre los 2 parámetros
  (if (and (< ScaleZ 3.0) (> ScaleZ 0.0))
    (`SceneComponent.SetWorldScale3D` Arrow (`KismetMathLibrary.MakeVector` 1.0 1.0 ScaleZ))
    (else
      ; Invertir dirección del incremento de la escalaZ si se sale de los parámetros
      (`|VariableSetRef` ScaleSpped (* ScaleSpped -1.0)))))

(fn `UserConstructionScript`)